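; Game mode for an infinite terrain game that spawns chained terrain tiles and keeps the score.
; BeginPlay calls PopulateBoundsVolumePool, then spawns the initial run of tiles.
; SpawnTile hands each new Tile_BP the shared nav mesh bounds volume pool and takes its arrow transform as the next spawn point.
; IncrementScore adds one to Score.
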(event `self.ReceiveBeginPlay`
  (`self.PopulateBoundsVolumePool`)
  (for _ (range 4)
    (`self.SpawnTile`)))

(fn `IncrementScore`
  (`/Engine/EditorBlueprintResources/StandardMacros.IncrementInt` (`self.Score`)))

(fn `SpawnTile`
  (bind _returnvalue (`|SpawnActorFromClass` "/Game/Dynamic/Terrain/Tile_BP.Tile_BP_C" (`self.SpawnTransform`) "Undefined" "OverrideRootScale" null null))
  (bind _output_get (set `self.Tile_BP` _returnvalue))
  (`Tile.SetPool` _output_get (`self.NavMeshBoundsVolumePool`))
  (set `self.SpawnTransform` (`/Game/Dynamic/Terrain/Tile_BP.GetArrowTransform` _output_get)))

(fn `UserConstructionScript`)