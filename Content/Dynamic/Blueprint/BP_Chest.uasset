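; Purchasable loot chest that gives a random weapon, priced in tiers by the game mode's Score when constructed and shown on a cost text.
; Box overlap with the player toggles custom depth on the chest meshes as a highlight.
; Open deducts the cost without a funds check, spawns the weapon at SpawnPoint, and removes the price text and interaction collision.
; A looping timer swings the lid open in small roll steps.
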(event `self.ReceiveBeginPlay`
  (bind _asue_4asp_character (cast `/Game/Dynamic/NPC/CharacterBlueprint/Ue4ASP_Character` (`GameplayStatics.GetPlayerCharacter` 0)))
  (set `self.Character` _asue_4asp_character)
  (`self.RenderCustomDepth?` false))

(event `RotateDoor`
  (bind _pivotdoor (`self.PivotDoor`))
  (bind (_relativerotation_roll _relativerotation_pitch _relativerotation_yaw) (`KismetMathLibrary.BreakRotator` (`SceneComponent.RelativeRotation` _pivotdoor)))
  (bind _returnvalue (+ _relativerotation_roll 1.0))
  (if (>= _returnvalue 40.0)
    (`KismetSystemLibrary.K2_ClearAndInvalidateTimerHandle` (`self.RotateHandle`))
    (else
      (`SceneComponent.K2_SetRelativeRotation` _pivotdoor (`KismetMathLibrary.MakeRotator` _returnvalue _relativerotation_pitch _relativerotation_yaw) false false))))

(event `self.Open`
  (bind _possibleweap (`self.PossibleWeap`))
  (bind _character (`self.Character`))
  (bind _returnvalue (`KismetSystemLibrary.K2_SetTimer` null "RotateDoor" 0.04 true))
  (set `self.RotateHandle` _returnvalue)
  (`self.RotateDoor`)
  (set `PrimitiveComponent.bGenerateOverlapEvents` false (`self.Box`))
  (`PrimitiveComponent.SetCollisionResponseToChannel` (`self.chest_chest1`) "ECC_GameTraceChannel4" "ECR_Ignore")
  (`PrimitiveComponent.SetCollisionResponseToChannel` (`self.chest_lock`) "ECC_GameTraceChannel4" "ECR_Ignore")
  (`PrimitiveComponent.SetCollisionResponseToChannel` (`self.chest_door`) "ECC_GameTraceChannel4" "ECR_Ignore")
  (`self.RenderCustomDepth?` false)
  (bind _returnvalue_2 (`|SpawnActorFromClass` (`|GetArrayItem` _possibleweap (`KismetMathLibrary.RandomIntegerInRange` 0 (- (`KismetArrayLibrary.Array_Length` _possibleweap) 1))) (`KismetMathLibrary.MakeTransform` (`SceneComponent.K2_GetComponentLocation` (`self.SpawnPoint`))) "AlwaysSpawn" "OverrideRootScale" null null))
  (`self.K2_AttachToComponent` _returnvalue_2 (`self.SpawnPoint`) "None" "KeepWorld" "KeepWorld" "KeepWorld" true)
  (`ActorComponent.K2_DestroyComponent` (`self.COsttt`))
  (set `Mannequin.CurrentMoney` (- (`Mannequin.CurrentMoney` _character) (`self.CostChest`)) _character)
  (`GameplayStatics.PlaySound2D` "/Game/Sounds/DoorOpenSquezy.DoorOpenSquezy"))

(event `self.Box.OnComponentBeginOverlap`
  (params (OverlappedComponent :type "PrimitiveComponent Object Reference") (OtherActor :type "Actor Object Reference") (OtherComp :type "PrimitiveComponent Object Reference") (OtherBodyIndex :type Integer) (bFromSweep :type Boolean) (SweepResult :type "HitResult Structure (by ref)"))
  (if (== OtherActor (`self.Character`))
    (`self.RenderCustomDepth?` true)))

(event `self.Box.OnComponentEndOverlap`
  (params (OverlappedComponent :type "PrimitiveComponent Object Reference") (OtherActor :type "Actor Object Reference") (OtherComp :type "PrimitiveComponent Object Reference") (OtherBodyIndex :type Integer))
  (if (== OtherActor (`self.Character`))
    (`self.RenderCustomDepth?` false)))

(fn `RenderCustomDepth?`
  (params (Value :type Boolean))
  (`PrimitiveComponent.SetRenderCustomDepth` (`self.chest_chest1`) Value)
  (`PrimitiveComponent.SetRenderCustomDepth` (`self.chest_lock`) Value)
  (`PrimitiveComponent.SetRenderCustomDepth` (`self.chest_door`) Value))

(fn `UserConstructionScript`
  (bind _score (`InfiniteTerrainGameMode.Score` (cast `/Game/Dynamic/InfiniteTerrainGameMode_BP` (`GameplayStatics.GetGameMode`) :!pure true)))
  (if (>= _score 2)
    (set `self.CostChest` 1250.0))
  (if (>= _score 5)
    (set `self.CostChest` 2000.0))
  (if (>= _score 9)
    (set `self.CostChest` 4000.0))
  (`TextRenderComponent.K2_SetText` (`self.COsttt`) (`|FormatText` "${Cost}" (`KismetTextLibrary.Conv_DoubleToText` (`self.CostChest`) "HalfToEven"))))