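; Boss tile for infinite terrain that, when prop spawning is enabled, spawns a guarded AI boss plus randomly placed props and pickups, and removes its back wall.
; Player entry into LockVolume opens the barrier, increments the game mode score once and teleports the boss to its spawn point.
; Leaving that volume relocks the barrier.
; Reaching DeleteVolume makes the game mode spawn another tile, then destroys this one.
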(event `self.ReceiveBeginPlay`
  (`self.Lock`)
  (if (`self.ShouldSpawnProps?`)
    (bind _returnvalue (`AIBlueprintHelperLibrary.SpawnAIFromClass` "/Game/Dynamic/NPC/CharacterBlueprint/AICharacter3.AICharacter3_C" "/Game/Dynamic/NPC/AI/GuardBehaviorTree.GuardBehaviorTree" (`SceneComponent.K2_GetComponentLocation` (`self.BossSpawnPOINT`)) (struct) true))
    (set `self.BossRef` _returnvalue)
    (`self.PlaceActors` "/Game/Dynamic/Terrain/Props/BP_Box.BP_Box_C" 1 5 100.0 1.0 1.5)
    (`self.PlaceActors` "/Game/Dynamic/Terrain/Props/BP_Canister.BP_Canister_C" 1 7 50.0 1.0 1.5)
    (`self.PlaceActors` "/Game/Dynamic/Terrain/Props/BP_Container.BP_Container_C" 0 4 400.0)
    (`self.PlaceActors` "/Game/Dynamic/Terrain/Props/BP_Rock01.BP_Rock01_C" 0 4 200.0 1.0 5.0)
    (`self.PlaceActors` "/Game/Dynamic/Terrain/Props/BP_Rock02.BP_Rock02_C" 0 4 300.0 1.0 5.0)
    (`self.PlaceActors` "/Game/Dynamic/Terrain/Props/BP_Rock03.BP_Rock03_C" 0 4 300.0 1.0 5.0)
    (`self.PlaceActors` "/Game/Dynamic/Terrain/Props/BP_SandBags.BP_SandBags_C" 0 3 250.0)
    (`self.PlaceActors` "/Game/Dynamic/Blueprint/BP_HealthPickup.BP_HealthPickup_C" 2 2 100.0)
    (`self.PlaceActors` "/Game/Dynamic/Blueprint/BP_AmmoPickup.BP_AmmoPickup_C" 2 2 100.0)))

(event `self.LockVolume.OnComponentBeginOverlap`
  (params (OverlappedComponent :type "PrimitiveComponent Object Reference") (OtherActor :type "Actor Object Reference") (OtherComp :type "PrimitiveComponent Object Reference") (OtherBodyIndex :type Integer) (bFromSweep :type Boolean) (SweepResult :type "HitResult Structure (by ref)"))
  (`self.IsActorPlayer` OtherActor
    (:`True`
      (`self.UnLock`)
      (`self.NewTileEntered`)
      (`self.K2_SetActorLocation` (`self.BossRef`) (`SceneComponent.K2_GetComponentLocation` (`self.BossSpawnPOINT`)) false false))))

(event `self.LockVolume.OnComponentEndOverlap`
  (params (OverlappedComponent :type "PrimitiveComponent Object Reference") (OtherActor :type "Actor Object Reference") (OtherComp :type "PrimitiveComponent Object Reference") (OtherBodyIndex :type Integer))
  (`self.IsActorPlayer` OtherActor
    (:`True`
      (`self.Lock`))))

(event `self.DeleteVolume.OnComponentBeginOverlap`
  (params (OverlappedComponent :type "PrimitiveComponent Object Reference") (OtherActor :type "Actor Object Reference") (OtherComp :type "PrimitiveComponent Object Reference") (OtherBodyIndex :type Integer) (bFromSweep :type Boolean) (SweepResult :type "HitResult Structure (by ref)"))
  (`self.IsActorPlayer` OtherActor
    (:`True`
      (bind _asinfinite_terrain_game_mode_bp (cast `/Game/Dynamic/InfiniteTerrainGameMode_BP` (`GameplayStatics.GetGameMode`)))
      (`/Game/Dynamic/InfiniteTerrainGameMode_BP.SpawnTile` _asinfinite_terrain_game_mode_bp)
      (`self.K2_DestroyActor`))))

(fn `GetArrowTransform`
  (returns (ArrowTransform :type "Transform Structure"))
  (return (`SceneComponent.K2_GetComponentToWorld` (`self.Arrow`))))

(fn `Lock`
  (`PrimitiveComponent.SetCollisionEnabled` (`self.Barrier`) "QueryAndPhysics")
  (`PrimitiveComponent.SetMaterial` (`self.Barrier`) 0 "/Game/Dynamic/Terrain/RedBarrier_MI.RedBarrier_MI"))

(fn `NewTileEntered`
  (if (not (`self.HasEnteredTile`))
    (bind _asinfinite_terrain_game_mode_bp (cast `/Game/Dynamic/InfiniteTerrainGameMode_BP` (`GameplayStatics.GetGameMode`)))
    (`/Game/Dynamic/InfiniteTerrainGameMode_BP.IncrementScore` _asinfinite_terrain_game_mode_bp)
    (set `self.HasEnteredTile` true)))

(fn `UnLock`
  (`PrimitiveComponent.SetCollisionEnabled` (`self.Barrier`) "QueryOnly")
  (`PrimitiveComponent.SetMaterial` (`self.Barrier`) 0 "/Game/Dynamic/Terrain/RedBarrier_MI.RedBarrier_MI"))

(fn `UserConstructionScript`
  (bind _backwall (`self.BackWall`))
  (if (`self.ShouldSpawnProps?`)
    (`SceneComponent.SetHiddenInGame` _backwall true false)
    (`PrimitiveComponent.SetCollisionEnabled` _backwall "NoCollision")
    (else
      (`SceneComponent.SetHiddenInGame` _backwall false false)
      (`PrimitiveComponent.SetCollisionEnabled` _backwall "QueryAndPhysics"))))