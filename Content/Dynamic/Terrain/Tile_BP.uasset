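; Terrain tile actor for an infinite terrain mode, with a barrier that switches between locked (red, colliding) and unlocked (green, no collision).
; The barrier starts locked, opens while the player overlaps LockVolume, and on exit relocks and asks InfiniteTerrainGameMode_BP to spawn a tile.
; Player overlap with DeleteVolume destroys the tile, and GetArrowTransform exposes the Arrow's world transform.
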(event `self.ReceiveBeginPlay`
  (`self.Lock`))

(event `self.LockVolume.OnComponentBeginOverlap`
  (params (OverlappedComponent :type "PrimitiveComponent Object Reference") (OtherActor :type "Actor Object Reference") (OtherComp :type "PrimitiveComponent Object Reference") (OtherBodyIndex :type Integer) (bFromSweep :type Boolean) (SweepResult :type "HitResult Structure (by ref)"))
  (`self.IsActorPlayer` OtherActor
    (:`True`
      (`self.UnLock`))))

(event `self.LockVolume.OnComponentEndOverlap`
  (params (OverlappedComponent :type "PrimitiveComponent Object Reference") (OtherActor :type "Actor Object Reference") (OtherComp :type "PrimitiveComponent Object Reference") (OtherBodyIndex :type Integer))
  (`self.IsActorPlayer` OtherActor
    (:`True`
      (`self.Lock`)
      (bind _asinfinite_terrain_game_mode_bp (cast `/Game/Dynamic/InfiniteTerrainGameMode_BP` (`GameplayStatics.GetGameMode`)))
      (`/Game/Dynamic/InfiniteTerrainGameMode_BP.SpawnTile` _asinfinite_terrain_game_mode_bp))))

(event `self.DeleteVolume.OnComponentBeginOverlap`
  (params (OverlappedComponent :type "PrimitiveComponent Object Reference") (OtherActor :type "Actor Object Reference") (OtherComp :type "PrimitiveComponent Object Reference") (OtherBodyIndex :type Integer) (bFromSweep :type Boolean) (SweepResult :type "HitResult Structure (by ref)"))
  (`self.IsActorPlayer` OtherActor
    (:`True`
      (`self.K2_DestroyActor`))))

(fn `GetArrowTransform`
  (returns (ArrowTransform :type "Transform Structure"))
  (return (`SceneComponent.K2_GetComponentToWorld` (`self.Arrow`))))

(fn `Lock`
  (`PrimitiveComponent.SetCollisionEnabled` (`self.Barrier`) "QueryAndPhysics")
  (`PrimitiveComponent.SetMaterial` (`self.Barrier`) 0 "/Game/Dynamic/Terrain/RedBarrier_MI.RedBarrier_MI"))

(fn `UnLock`
  (`PrimitiveComponent.SetCollisionEnabled` (`self.Barrier`) "NoCollision")
  (`PrimitiveComponent.SetMaterial` (`self.Barrier`) 0 "/Game/Dynamic/Terrain/GreenBarrier_MI.GreenBarrier_MI"))

(fn `UserConstructionScript`)