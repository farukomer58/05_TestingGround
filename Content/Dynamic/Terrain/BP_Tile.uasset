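; Terrain tile for an infinite-terrain mode that scatters props, pickups and score-tiered AI on spawn when ShouldSpawnProps is set, otherwise showing a back wall.
; The player overlapping LockVolume turns the barrier green and passable and increments the GameMode score once; leaving relocks it.
; Reaching DeleteVolume has the GameMode spawn the next tile, or a one-time boss tile at high score, then destroys this tile.
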(event `self.ReceiveBeginPlay`
  (`self.Lock`)
  (if (`self.ShouldSpawnProps?`)
    (`self.SpawnAI`)
    (`self.PlaceActors` "/Game/Dynamic/Terrain/Props/BP_Box.BP_Box_C" 1 5 100.0 1.0 1.5)
    (`self.PlaceActors` "/Game/Dynamic/Terrain/Props/BP_Canister.BP_Canister_C" 1 7 50.0 1.0 1.5)
    (`self.PlaceActors` "/Game/Dynamic/Terrain/Props/BP_Container.BP_Container_C" 0 4 400.0)
    (`self.PlaceActors` "/Game/Dynamic/Terrain/Props/BP_Rock01.BP_Rock01_C" 0 4 200.0 1.0 5.0)
    (`self.PlaceActors` "/Game/Dynamic/Terrain/Props/BP_Rock02.BP_Rock02_C" 0 4 300.0 1.0 5.0)
    (`self.PlaceActors` "/Game/Dynamic/Terrain/Props/BP_Rock03.BP_Rock03_C" 0 4 300.0 1.0 5.0)
    (`self.PlaceActors` "/Game/Dynamic/Terrain/Props/BP_SandBags.BP_SandBags_C" 0 3 250.0)
    (`self.PlaceActors` "/Game/Dynamic/Blueprint/BP_Chest.BP_Chest_C" 1 1)
    (if (== (mod (`InfiniteTerrainGameMode.Score` (cast `/Game/Dynamic/InfiniteTerrainGameMode_BP` (`GameplayStatics.GetGameMode`) :!pure true)) 8) 0)
      (`self.PlaceActors` "/Game/Dynamic/Blueprint/BP_HealthPickup.BP_HealthPickup_C" 1 1 100.0))))

(event `self.LockVolume.OnComponentBeginOverlap`
  (params (OverlappedComponent :type "PrimitiveComponent Object Reference") (OtherActor :type "Actor Object Reference") (OtherComp :type "PrimitiveComponent Object Reference") (OtherBodyIndex :type Integer) (bFromSweep :type Boolean) (SweepResult :type "HitResult Structure (by ref)"))
  (`self.IsActorPlayer` OtherActor
    (:`True`
      (`self.UnLock`)
      (`self.NewTileEntered`))))

(event `self.LockVolume.OnComponentEndOverlap`
  (params (OverlappedComponent :type "PrimitiveComponent Object Reference") (OtherActor :type "Actor Object Reference") (OtherComp :type "PrimitiveComponent Object Reference") (OtherBodyIndex :type Integer))
  (`self.IsActorPlayer` OtherActor
    (:`True`
      (`self.Lock`))))

(event `self.DeleteVolume.OnComponentBeginOverlap`
  (params (OverlappedComponent :type "PrimitiveComponent Object Reference") (OtherActor :type "Actor Object Reference") (OtherComp :type "PrimitiveComponent Object Reference") (OtherBodyIndex :type Integer) (bFromSweep :type Boolean) (SweepResult :type "HitResult Structure (by ref)"))
  (`self.IsActorPlayer` OtherActor
    (:`True`
      (bind _asinfinite_terrain_game_mode_bp (cast `/Game/Dynamic/InfiniteTerrainGameMode_BP` (`GameplayStatics.GetGameMode`)))
      (if (>= (`InfiniteTerrainGameMode.Score` _asinfinite_terrain_game_mode_bp) 12)
        (if (`/Game/Dynamic/InfiniteTerrainGameMode_BP.SpawnedBossTile` _asinfinite_terrain_game_mode_bp)
          (`self.K2_DestroyActor`)
          (else
            (`/Game/Dynamic/InfiniteTerrainGameMode_BP.SpawnBossTile` _asinfinite_terrain_game_mode_bp)
            (`self.K2_DestroyActor` self)))
        (else
          (`/Game/Dynamic/InfiniteTerrainGameMode_BP.SpawnTile` _asinfinite_terrain_game_mode_bp)
          (`self.K2_DestroyActor` self))))))

(fn `GetArrowTransform`
  (returns (ArrowTransform :type "Transform Structure"))
  (return (`SceneComponent.K2_GetComponentToWorld` (`self.Arrow`))))

(fn `Lock`
  (`PrimitiveComponent.SetCollisionEnabled` (`self.Barrier`) "QueryAndPhysics")
  (`PrimitiveComponent.SetMaterial` (`self.Barrier`) 0 "/Game/Dynamic/Terrain/RedBarrier_MI.RedBarrier_MI"))

(fn `NewTileEntered`
  (if (not (`self.HasEnteredTile`))
    (bind _asinfinite_terrain_game_mode_bp (cast `/Game/Dynamic/InfiniteTerrainGameMode_BP` (`GameplayStatics.GetGameMode`)))
    (`/Game/Dynamic/InfiniteTerrainGameMode_BP.IncrementScore` _asinfinite_terrain_game_mode_bp)
    (set `self.HasEnteredTile` true)))

(fn `SpawnAI`
  (bind _asinfinite_terrain_game_mode_bp (cast `/Game/Dynamic/InfiniteTerrainGameMode_BP` (`GameplayStatics.GetGameMode`) :!pure true))
  (bind _score (`InfiniteTerrainGameMode.Score` _asinfinite_terrain_game_mode_bp))
  (if (>= _score 12)
    _
    (elif (>= _score 5)
      (if (>= (`InfiniteTerrainGameMode.Score` _asinfinite_terrain_game_mode_bp) 8)
        (`self.PlaceAIPawns` "/Game/Dynamic/NPC/CharacterBlueprint/AICharacter0.AICharacter0_C" 1 1 100.0)
        (`self.PlaceAIPawns` "/Game/Dynamic/NPC/CharacterBlueprint/AICharacter1.AICharacter1_C" 1 2 100.0)
        (`self.PlaceAIPawns` "/Game/Dynamic/NPC/CharacterBlueprint/AICharacter2.AICharacter2_C" 1 2 100.0)
        (`self.PlaceActors` "/Game/Dynamic/Blueprint/BP_Chest.BP_Chest_C" 1 3)
        (else
          (`self.PlaceAIPawns` "/Game/Dynamic/NPC/CharacterBlueprint/AICharacter0.AICharacter0_C" 1 3 100.0)
          (`self.PlaceAIPawns` "/Game/Dynamic/NPC/CharacterBlueprint/AICharacter1.AICharacter1_C" 1 3 100.0)))
      (else
        (`self.PlaceAIPawns` "/Game/Dynamic/NPC/CharacterBlueprint/AICharacter0.AICharacter0_C" 1 4 100.0)))))

(fn `UnLock`
  (`PrimitiveComponent.SetCollisionEnabled` (`self.Barrier`) "NoCollision")
  (`PrimitiveComponent.SetMaterial` (`self.Barrier`) 0 "/Game/Dynamic/Terrain/GreenBarrier_MI.GreenBarrier_MI"))

(fn `UserConstructionScript`
  (bind _backwall (`self.BackWall`))
  (if (`self.ShouldSpawnProps?`)
    (`SceneComponent.SetHiddenInGame` _backwall true false)
    (`PrimitiveComponent.SetCollisionEnabled` _backwall "NoCollision")
    (else
      (`SceneComponent.SetHiddenInGame` _backwall false false)
      (`PrimitiveComponent.SetCollisionEnabled` _backwall "QueryAndPhysics"))))