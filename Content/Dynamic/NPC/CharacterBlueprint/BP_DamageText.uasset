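; BP_DamageText is a short-lived floating damage number actor that displays DamageAmount and destroys itself after one second.
; BeginPlay sets the text and picks random upward and sideways offsets.
; Every tick it turns in pitch and yaw to face ActorToLookAt and calls MoveComponentTo on its root, targeting its current location plus those offsets, so the number drifts up and to one side.
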(event `self.ReceiveBeginPlay`
  (`TextRenderComponent.K2_SetText` (`self.DamageAmountText`) (`KismetTextLibrary.Conv_DoubleToText` (`self.DamageAmount`) "HalfToEven" true 1 324 0 0))
  (set `self.RandomUp` (`KismetMathLibrary.RandomIntegerInRange` 30 80))
  (set `self.RandomLR` (`KismetMathLibrary.RandomIntegerInRange` -30 30))
  (`KismetSystemLibrary.Delay` 1.0)
  (`self.K2_DestroyActor`))

(event `self.ReceiveTick`
  (params (DeltaSeconds :type "Float (single-precision)"))
  (bind (_returnvalue_x _returnvalue_y _returnvalue_z) (`KismetMathLibrary.BreakVector` (`self.K2_GetActorLocation`)))
  (bind (_returnvalue_roll _returnvalue_pitch _returnvalue_yaw) (`KismetMathLibrary.BreakRotator` (`KismetMathLibrary.FindLookAtRotation` (`self.K2_GetActorLocation`) (`self.K2_GetActorLocation` (`self.ActorToLookAt`)))))
  (`self.K2_SetActorRotation` (`KismetMathLibrary.MakeRotator` 0.0 _returnvalue_pitch _returnvalue_yaw))
  (`KismetSystemLibrary.MoveComponentTo` (`self.DefaultSceneRoot`) (+ (`KismetMathLibrary.MakeVector` _returnvalue_x _returnvalue_y (+ _returnvalue_z (`KismetMathLibrary.Conv_IntToDouble` (`self.RandomUp`)))) (* (`self.GetActorRightVector`) (`self.RandomLR`))) (`self.K2_GetActorRotation`) false false 0.5))

(fn `UserConstructionScript`)