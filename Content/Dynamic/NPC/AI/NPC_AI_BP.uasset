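; AI controller for guard NPCs that runs a patrol blackboard and guard behavior tree.
; On BeginPlay it also caches the controlled pawn as a Ue4ASP_Character.
; Perception updates treat actors without the "Enemy" tag as targets, writing them to the blackboard's enemy key when sensed.
; When such a target is no longer sensed, it clears the key and focus and prints a debug message.
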(event `self.ReceiveBeginPlay`
  (`self.UseBlackboard` "/Game/Dynamic/NPC/AI/PatrolBlackBoard.PatrolBlackBoard")
  (`self.RunBehaviorTree` "/Game/Dynamic/NPC/AI/GuardBehaviorTree.GuardBehaviorTree")
  (bind _asue_4asp_character (cast `/Game/Dynamic/NPC/CharacterBlueprint/Ue4ASP_Character` (`self.K2_GetPawn`)))
  (set `self.ControlledPawn` _asue_4asp_character))

(event `self.AIPerception.OnTargetPerceptionUpdated`
  (params (Actor :type "Actor Object Reference") (Stimulus :type "AIStimulus Structure"))
  (bind _returnvalue (`AIBlueprintHelperLibrary.GetBlackboard` null))
  (bind _enemykey (`self.EnemyKey`))
  (if (`self.ActorHasTag` Actor "Enemy")
    _
    (elif (`.bSuccessfullySensed` (break `AIStimulus` Stimulus))
      (`BlackboardComponent.SetValueAsObject` _returnvalue _enemykey Actor)
      (else
        (`BlackboardComponent.ClearValue` _returnvalue _enemykey)
        (`KismetSystemLibrary.PrintString` "NO ENEMY" true true (struct :`R` 1.0 :`B` 0.008304 :`A` 1.0))
        (`self.K2_ClearFocus`)))))

(fn `UserConstructionScript`)